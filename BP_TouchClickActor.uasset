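; BP_TouchClickActor is an actor that responds to mouse clicks and mobile touches, apparently as an input test.
; A click spawns an explosion emitter at the eye viewpoint location taken from Camera and prints a debug message, while a touch only prints its own message.
; Both paths then set the TouchClick component's relative location with a zero offset, leaving it in place.
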(event EventBeginPlay)

(event Collision|EventActorBeginOverlap
  (params (OtherActor :type Actor%20Object%20Reference)))

(event EventTick
  (params (DeltaSeconds :type Float%20%28single-precision%29)))

(event MouseInput|EventActorOnClicked
  (params (ButtonPressed :type Key%20Structure :default "None"))
  (Effects|SpawnEmitteratLocation "/Game/StarterContent/Particles/P_Explosion.P_Explosion" (.OutLocation (Actor|GetActorEyesViewPoint (Variables|Default|GetCamera))))
  (Development|PrintString "Mouse Clicked")
  (Transformation|SetRelativeLocation (Variables|Default|GetTouchClick) (+ (Variables|/Script/Engine.SceneComponent|GetRelativeLocation (Variables|Default|GetTouchClick)) "0, 0,0.000000") false false))

(event EventActorOnInputTouchBegin
  (params (FingerIndex :type ETouchIndex%20Enum :default "Touch1"))
  (Development|PrintString "Mobile Clicked")
  (Transformation|SetRelativeLocation (Variables|Default|GetTouchClick) (+ (Variables|/Script/Engine.SceneComponent|GetRelativeLocation (Variables|Default|GetTouchClick)) "0, 0,0.000000") false false))

(fn ConstructionScript)